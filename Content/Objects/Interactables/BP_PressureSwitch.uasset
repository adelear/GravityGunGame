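; BP_PressureSwitch is a floor pressure plate that activates a linked bridge when an actor overlaps it.
; Actors tagged "Light" do not trigger it and instead show a too-light message on the player's UI.
; A valid overlap calls SwitchActivated on the bridge and lowers the switch mesh with a timeline.
; Any end overlap, regardless of tag, deactivates the bridge and reverses the timeline.
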(event Custom|PlayerRef
  (bind _outactors (Actor|GetAllActorsOfClass "/Game/FirstPerson/Blueprints/BP_FirstPersonCharacter.BP_FirstPersonCharacter_C"))
  (Variables|Default|SetPlayer (Utilities|Array|Get(acopy) _outactors)))

(event EventBeginPlay
  (CallFunction|PlayerRef))

(event Collision|EventActorBeginOverlap
  (params (OtherActor :type Actor%20Object%20Reference))
  (if (not (Actor|ActorHasTag OtherActor "Light"))
    (Variables|/Game/FirstPerson/UI/W_PickUp.W_PickUp_C|SetMessage (Variables|/Game/FirstPerson/Blueprints/BP_FirstPersonCharacter.BP_FirstPersonCharacter_C|GetMessageUI (Variables|Default|GetPlayer)) "")
    (Default|SwitchActivated (Variables|Default|GetBridgeToActivate))
    (bind _switchposition (Timeline|SwitchActivate Play)
      (:Update
        (Transformation|SetRelativeLocation (Variables|Default|GetSwitch) (Math|Vector|MakeVector 0.0 0.0 _switchposition) false false)))
    (else
      (Variables|/Game/FirstPerson/UI/W_PickUp.W_PickUp_C|SetMessage (Variables|/Game/FirstPerson/Blueprints/BP_FirstPersonCharacter.BP_FirstPersonCharacter_C|GetMessageUI (Variables|Default|GetPlayer)) "This object is too light to trigger this plate..."))))

(event Collision|EventActorEndOverlap
  (params (OtherActor :type Actor%20Object%20Reference))
  (Variables|/Game/FirstPerson/UI/W_PickUp.W_PickUp_C|SetMessage (Variables|/Game/FirstPerson/Blueprints/BP_FirstPersonCharacter.BP_FirstPersonCharacter_C|GetMessageUI (Variables|Default|GetPlayer)) "")
  (Default|SwitchDeactivated (Variables|Default|GetBridgeToActivate))
  (Development|PrintString "Bridge Closing")
  (bind _switchposition (Timeline|SwitchActivate Reverse)
    (:Update
      (Transformation|SetRelativeLocation (Variables|Default|GetSwitch) (Math|Vector|MakeVector 0.0 0.0 _switchposition) false false))))

(fn ConstructionScript)